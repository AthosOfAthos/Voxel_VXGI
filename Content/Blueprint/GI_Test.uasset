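; Test actor that generates a random voxel chunk on the server and renders it as instanced static meshes.
; After a short delay on BeginPlay, the authority fills ChunkData with random zeros and ones, then enables replication.
; The ChunkData RepNotify calls UpdateChunk, which maps each flat array index to a cell in a 10x10x10 grid and adds an instance for every filled cell.
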(event Custom|UpdateChunk
  (for _index (range 0 999)
    (if (> (Utilities|Array|Get(acopy) (Variables|Default|GetchunkData) _index) 0)
      (Components|InstancedStaticMesh|AddInstance (Variables|Default|GetInstancedStaticMesh) (Math|Transform|MakeTransform (Math|Vector|MakeVector (Math|Conversions|ToFloat(Integer) (* (Math|Integer|%(Integer) _index 10) 100)) (Math|Conversions|ToFloat(Integer) (* (Math|Integer|%(Integer) (/ _index 10) 10) 100)) (Math|Conversions|ToFloat(Integer) (* (/ _index 100) 100))))))))

(event EventBeginPlay
  (Networking|SwitchHasAuthority
    (:Authority
      (Utilities|FlowControl|Delay 2.0)
      (for _index (range 0 999)
        (Utilities|Array|Add (Variables|Default|GetchunkData) (Math|Random|RandomIntegerinRange 0 1)))
      (Networking|SetReplicates true))))

(fn ConstructionScript)

(fn OnRepChunkData
  (CallFunction|UpdateChunk))